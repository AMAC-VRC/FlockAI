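; Flocking agent Blueprint that computes a boids-style steering vector in CalculateNewMoveVector.
; Agents overlapping VisionSphere supply alignment, cohesion and distance-scaled separation, each weighted in the final sum.
; Overlapping Stimulus actors add unweighted terms: negatives combine into repulsion scaled by the strongest, while only the positive with the best value-to-distance ratio attracts.
; The result becomes NewMoveVector; a component-printing debug helper is left unwired.
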(event EventCalculateNewMoveVector
  (CallFunction|ResetComponents)
  (Variables|AI|SetNeighbourhood (Collision|GetOverlappingActors (Variables|Default|GetVisionSphere) "/Script/FlockAI.Agent" :!class /Script/Engine.PrimitiveComponent))
  ;[1 1 1] Compute Alignment Component Vector
  (for _array_element (Variables|AI|GetNeighbourhood)
    (bind _asagent (Utilities|Casting|CastToAgent _array_element))
    (Variables|AI|SetAlignmentComponent (+ (Math|Vector|Normalize (Variables|/Script/FlockAI.Agent|GetCurrentMoveVector _asagent)) (Variables|AI|GetAlignmentComponent))))
  (Variables|AI|SetAlignmentComponent (Math|Vector|Normalize (Variables|AI|GetAlignmentComponent)))
  (Utilities|Array|RemoveItem (Variables|AI|GetNeighbourhood) self)
  (if (> (Utilities|Array|Length (Variables|AI|GetNeighbourhood)) 0)
    ;[1 1 1] Compute Cohesion Component Vector
    (for _array_element_2 (Variables|AI|GetNeighbourhood)
      (Variables|AI|SetCohesionComponent (+ (- (Transformation|GetActorLocation _array_element_2) (Transformation|GetActorLocation)) (Variables|AI|GetCohesionComponent))))
    (Variables|AI|SetCohesionComponent (/ (/ (Variables|AI|GetCohesionComponent) (Math|Conversions|ToFloat(Integer) (Utilities|Array|Length (Variables|AI|GetNeighbourhood)))) 1e+02))
    ;[1 1 1] Compute Separation Component Vector
    (for _array_element_3 (Variables|AI|GetNeighbourhood)
      (Variables|AI|SetSeparationComponent (+ (/ (Math|Vector|Normalize (- (Transformation|GetActorLocation) (Transformation|GetActorLocation _array_element_3))) (Math|Float|Absolute(Float) (- (Math|Vector|VectorLength (- (Transformation|GetActorLocation) (Transformation|GetActorLocation _array_element_3))) (* 2 (Variables|Default|GetAgentPhysicalRadius))))) (Variables|AI|GetSeparationComponent))))
    (Variables|AI|SetSeparationComponent (+ (* (Variables|AI|GetSeparationComponent) 1e+02) (* (* (Variables|AI|GetSeparationComponent) 1e+02) (/ 5.0 (Math|Conversions|ToFloat(Integer) (Utilities|Array|Length (Variables|AI|GetNeighbourhood))))))))
  (for _array_element_4 (Collision|GetOverlappingActors (Variables|Default|GetVisionSphere) 0 :!class /Script/Engine.PrimitiveComponent)
    (bind _asstimulus (Utilities|Casting|CastToStimulus _array_element_4))
    (if (< (Variables|/Script/FlockAI.Stimulus|GetValue _asstimulus) 0.0)
      ;[1 1 1] Compute Negative Stimuli Component Vector
      (Variables|AI|SetNegativeStimuliComponent (+ (* (* (/ (Math|Vector|Normalize (- (Transformation|GetActorLocation _asstimulus) (Transformation|GetActorLocation))) (Math|Float|Absolute(Float) (- (Math|Vector|VectorLength (- (Transformation|GetActorLocation _asstimulus) (Transformation|GetActorLocation))) (Variables|Default|GetAgentPhysicalRadius)))) 1e+02) (Variables|/Script/FlockAI.Stimulus|GetValue _asstimulus)) (Variables|AI|GetNegativeStimuliComponent)))
      (Variables|AI|SetNegativeStimuliMaxFactor (Math|Float|Max(Float) (Variables|AI|GetNegativeStimuliMaxFactor) (Math|Vector|VectorLength (* (* (/ (Math|Vector|Normalize (- (Transformation|GetActorLocation _asstimulus) (Transformation|GetActorLocation))) (Math|Float|Absolute(Float) (- (Math|Vector|VectorLength (- (Transformation|GetActorLocation _asstimulus) (Transformation|GetActorLocation))) (Variables|Default|GetAgentPhysicalRadius)))) 1e+02) (Variables|/Script/FlockAI.Stimulus|GetValue _asstimulus)))))
      (else
        ;[1 1 1] Compute Positive Stimuli Component Vector
        (if (> (/ (Variables|/Script/FlockAI.Stimulus|GetValue _asstimulus) (Math|Vector|VectorLength (- (Transformation|GetActorLocation _asstimulus) (Transformation|GetActorLocation)))) (Variables|AI|GetPositiveStimuliMaxFactor))
          (Variables|AI|SetPositiveStimuliComponent (* (Math|Vector|Normalize (- (Transformation|GetActorLocation _asstimulus) (Transformation|GetActorLocation))) (Variables|/Script/FlockAI.Stimulus|GetValue _asstimulus)))
          (Variables|AI|SetPositiveStimuliMaxFactor (/ (Variables|/Script/FlockAI.Stimulus|GetValue _asstimulus) (Math|Vector|VectorLength (- (Transformation|GetActorLocation _asstimulus) (Transformation|GetActorLocation)))))))))
  (Variables|AI|SetNegativeStimuliComponent (* (Math|Vector|Normalize (Variables|AI|GetNegativeStimuliComponent)) (Variables|AI|GetNegativeStimuliMaxFactor)))
  ;[1 1 1] Compute Aggregation of Components
  (Variables|Default|SetNewMoveVector (+ (* (Variables|AI|GetAlignmentComponent) (Variables|Default|GetAlignmentWeight)) (* (Variables|AI|GetCohesionComponent) (Variables|Default|GetCohesionWeight)) (* (Variables|AI|GetSeparationComponent) (Variables|Default|GetSeparationWeight)) (Variables|AI|GetNegativeStimuliComponent) (Variables|AI|GetPositiveStimuliComponent))))

(fn ConstructionScript)

(fn ResetComponents
  (Variables|AI|SetAlignmentComponent "0, 0, 0")
  (Variables|AI|SetCohesionComponent "0, 0, 0")
  (Variables|AI|SetSeparationComponent "0, 0, 0")
  (Variables|AI|SetNegativeStimuliComponent "0, 0, 0")
  (Variables|AI|SetNegativeStimuliMaxFactor 0.0)
  (Variables|AI|SetPositiveStimuliComponent "0, 0, 0")
  (Variables|AI|SetPositiveStimuliMaxFactor 0.0))

(fn DebugComponents
  (Development|PrintString (Utilities|String|Append "Alignment: " (Utilities|String|ToString(Vector) (* (Variables|AI|GetAlignmentComponent) (Variables|Default|GetAlignmentWeight)))))
  (Development|PrintString (Utilities|String|Append "Cohesion: " (Utilities|String|ToString(Vector) (* (Variables|AI|GetCohesionComponent) (Variables|Default|GetCohesionWeight)))))
  (Development|PrintString (Utilities|String|Append "Separation:  " (Utilities|String|ToString(Vector) (* (Variables|AI|GetSeparationComponent) (Variables|Default|GetSeparationWeight)))))
  (Development|PrintString (Utilities|String|Append "NegativeStimuli:   " (Utilities|String|ToString(Vector) (Variables|AI|GetNegativeStimuliComponent))))
  (Development|PrintString (Utilities|String|Append "PositiveStimuli:   " (Utilities|String|ToString(Vector) (Variables|AI|GetPositiveStimuliComponent)))))